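; RightDoor is a door Blueprint that the first-person character opens and closes with the Use input.
; A UseTrigger overlap opens a Gate while the character is in range, letting Use presses through.
; A press prints a message if the door is Locked, otherwise toggles Opened.
; Opening plays the Ouverture sequence forward and closing plays it in reverse.
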(event OnComponentBeginOverlap(Usetrigger)
  (params (OverlappedComponent :type Primitive%20Component%20Object%20Reference) (OtherActor :type Actor%20Object%20Reference) (OtherComp :type Primitive%20Component%20Object%20Reference) (OtherBodyIndex :type Integer) (bFromSweep :type Boolean) (SweepResult :type Hit%20Result%20Structure%20%28by%20ref%29))
  ;[1 1 1] Use Door
  (Utilities|Casting|CastToFirstPersonCharacter OtherActor)
  (Utilities|FlowControl|Gate true) ; enters at Open
)

(event OnComponentEndOverlap(Usetrigger)
  (params (OverlappedComponent :type Primitive%20Component%20Object%20Reference) (OtherActor :type Actor%20Object%20Reference) (OtherComp :type Primitive%20Component%20Object%20Reference) (OtherBodyIndex :type Integer))
  ;[1 1 1] Use Door
  (Utilities|Casting|CastToFirstPersonCharacter OtherActor)
  (Utilities|FlowControl|Gate true) ; enters at Close
)

(event Custom|Open
  ;[1 1 1] Door Animation
  (Sequencer|Player|Play (Variables|/Script/ActorSequence.ActorSequenceComponent|GetSequencePlayer (Variables|Default|Getouverture)) :!class /Script/MovieScene.MovieSceneSequencePlayer)
  (Variables|Default|SetOpened true))

(event Custom|Close
  ;[1 1 1] Door Animation
  (Class|MovieSceneSequencePlayer|PlayReverse (Variables|/Script/ActorSequence.ActorSequenceComponent|GetSequencePlayer (Variables|Default|Getouverture)))
  (Variables|Default|SetOpened false))

(event Input|ActionEvents|InputActionUse
  (params (Key :type Key%20Structure :default "None"))
  ;[1 1 1] Use Door
  (:Pressed
    (Utilities|FlowControl|Gate true
      (:Exit
        (if (Variables|Default|GetLocked)
          (Development|PrintString "Locked")
          (elif (Variables|Default|GetOpened)
            (CallFunction|Close)
            (else
              (CallFunction|Open))))))))

(fn ConstructionScript)