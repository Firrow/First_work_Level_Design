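; Test NPC that walks a patrol route and reacts when it spots the first-person player character.
; PawnSensing triggers a debug "SPOTTED" print and shows the Attention "!" marker, hiding it after a fixed delay.
; The Patrol event uses AIMoveTo, waits for each point's Duration, then calls itself with that point's NextPoint until the chain ends.
; Sighting the player does not interrupt the patrol.
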(event OnSeePawn(PawnSensing)
  (params (Pawn :type Pawn%20Object%20Reference))
  (bind _attention (Variables|Default|GetAttention))
  ;[1 1 1] NPC Vision (DEBUG)
  (Utilities|Casting|CastToFirstPersonCharacter Pawn)
  (Development|PrintString "SPOTTED !!!!!" true true "(R=1.000000,G=0.028286,B=0.000000,A=1.000000)")
  (Rendering|SetVisibility _attention true false) ; Affiche "!"
  (Utilities|FlowControl|Delay 5.0)
  (Rendering|SetVisibility _attention false false) ; N'affiche plus "!"
)

(event Custom|Patrol
  (params (FirstPoint :type Patrol%20Point%20Object%20Reference))
  (bind _nextpoint (Variables|/Game/Test_Asset_Manon_Bonnot/Blueprints/PatrolPoint.PatrolPoint_C|GetNextPoint FirstPoint))
  ;[1 1 1] Patrol NextPoint
  (AI|AIMoveTo self "0, 0, 0" FirstPoint 5.0 false
    (:OnSuccess
      (Utilities|FlowControl|Delay (Variables|/Game/Test_Asset_Manon_Bonnot/Blueprints/PatrolPoint.PatrolPoint_C|GetDuration FirstPoint))
      ;[1 1 1] NextPoint exist ?
      (if (Utilities|IsValid _nextpoint)
        (CallFunction|Patrol _nextpoint)
        (else
          (Development|PrintString "Fin patrouille"))))))

(fn ConstructionScript)